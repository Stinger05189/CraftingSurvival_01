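; BP_Resource is a harvestable world resource that players deplete to gain materials.
; Each Harvest call lowers its remaining life, creating a WG_HarvestMeter on the player's harvest HUD if none exists and updating it with progress.
; When life runs out, it removes the meter, adds a random amount from the drop range to the player's Resources and destroys itself.
; Stopping harvesting removes the meter but keeps the reduced life.
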(event `/Game/MyStuff/Systems/HarvestSystem/BPI_Resource_Interactions.Harvest`
  (params (HarvestAmount :type "Float (single-precision)") (PlayerRef :type "/Game/MyStuff/Characters/MainCharacter Object Reference"))
  (set `self.PlayerRef` PlayerRef)
  (if (`KismetSystemLibrary.IsValid` (`self.HarvestUIRef`))
    (`self.CheckProgress` HarvestAmount)
    (else
      (bind _returnvalue (`|CreateWidget` "/Game/MyStuff/Systems/HarvestSystem/WG_HarvestMeter.WG_HarvestMeter_C"))
      (bind _output_get (set `self.HarvestUIRef` _returnvalue))
      (bind _returnvalue_2 (`PanelWidget.AddChild` (`/Game/MyStuff/Systems/HarvestSystem/WG_HarvestHUD.MainPanel` (`/Game/MyStuff/Characters/MainCharacter.WG_HarvestHudRef` (`self.PlayerRef`))) _output_get))
      (bind _ascanvas_panel_slot (cast `CanvasPanelSlot` _returnvalue_2))
      (`CanvasPanelSlot.SetAnchors` _ascanvas_panel_slot (make `Anchors` (0.4 0.8) (0.6 0.87)))
      (`CanvasPanelSlot.SetPosition` _ascanvas_panel_slot (0.0 0.0))
      (`CanvasPanelSlot.SetSize` _ascanvas_panel_slot (0.0 0.0))
      (`self.CheckProgress` HarvestAmount))))

(event `/Game/MyStuff/Systems/HarvestSystem/BPI_Resource_Interactions.UserStoppedHarvesting`
  (`Widget.RemoveFromParent` (`self.HarvestUIRef`))
  (set `self.HarvestUIRef` null))

(fn `CheckProgress`
  (params (HarvestAmount :type "Float (double-precision)"))
  (bind _output_get (set `self.HarvestCurrentLife` (- (`self.HarvestCurrentLife`) HarvestAmount)))
  (if (<= _output_get 0.0)
    (`self.ResourceDepleted`)
    (else
      (`/Game/MyStuff/Systems/HarvestSystem/WG_HarvestMeter.UpdateProgress` (`self.HarvestUIRef`) (`self.HarvestCurrentLife`) (`self.HarvestMaxLife`)))))

(fn `ResourceDepleted`
  (bind _playerref (`self.PlayerRef`))
  (bind _materialdropchance (`self.MaterialDropChance`))
  (`Widget.RemoveFromParent` (`self.HarvestUIRef`))
  (set `/Game/MyStuff/Characters/MainCharacter.Resources` (+ (`/Game/MyStuff/Characters/MainCharacter.Resources` _playerref) (`KismetMathLibrary.RandomIntegerInRange` (`|GetArrayItem` _materialdropchance) (`|GetArrayItem` _materialdropchance 1))) _playerref)
  (`self.K2_DestroyActor`))

(fn `UserConstructionScript`)